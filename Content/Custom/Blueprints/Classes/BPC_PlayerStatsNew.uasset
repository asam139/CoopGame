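; BPC_PlayerStatsNew is the player stats manager that links Health and Shield stats to their HUD bars.
; InitializeManager stores the player reference and runs stat setup, then OnStatsSetUp initializes a bar for each key in the Stats map using its StatValue.
; UpdateStat pushes a stat's CurrentValue to its bar, which GetBarForStat selects from the player's main widget.
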(event `InitializeManager`
  (params (NewParam :type "/Game/Custom/Blueprints/Characters/BP_PlayerCharacter Object Reference"))
  (set `self.PlayerRef` NewParam)
  (`self.SetupStats`))

(event `self.OnStatsSetUp`
  (bind _keys (`BlueprintMapLibrary.Map_Keys` (`self.Stats`)))
  (for _array_element _keys
    (`/Game/Custom/Blueprints/Widgets/W_StatBar.InitializeBar` (`self.GetBarForStat` _array_element) (`self.GetStat` _array_element))))

(event `self.UpdateStat`
  (params (Stat :type "/Game/Custom/Blueprints/Enums/E_Stats Enum" :default "NewEnumerator0"))
  (`/Game/Custom/Blueprints/Widgets/W_StatBar.UpdateStat` (`self.GetBarForStat` Stat) (`.CurrentValue` (`self.GetStat` Stat))))

(fn `GetBarForStat`
  (params (Stat :type "/Game/Custom/Blueprints/Enums/E_Stats Enum" :default "NewEnumerator0"))
  (returns (Bar :type "/Game/Custom/Blueprints/Widgets/W_StatBar Object Reference"))
  (bind _widgetmain (`/Game/Custom/Blueprints/Characters/BP_PlayerCharacter.WidgetMain` (`self.PlayerRef`)))
  (return (select `/Game/Custom/Blueprints/Enums/E_Stats` Stat :`NewEnumerator1` (`/Game/Custom/Blueprints/Widgets/W_Main.HealthBar` _widgetmain) :`NewEnumerator2` (`/Game/Custom/Blueprints/Widgets/W_Main.ShieldBar` _widgetmain))))