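; BP_LaunchPadMeshTest is a launch pad that throws the player straight up on contact and visually bounces when hit.
; A hit on the Cube uncrouches and launches a BP_PlayerCharacter, while a BP_Projectile triggers only the bounce.
; The bounce passes the impact point to a dynamic material, then a timeline drives its Impact vector along the hit normal, scaled by a curve and Bounciness.
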(event `self.ReceiveBeginPlay`
  ;[1 1 1] Set Material
  (bind _returnvalue (`PrimitiveComponent.CreateDynamicMaterialInstance` (`self.Cube`) 0 null))
  (set `self.Material` _returnvalue))

(event `self.Cube.OnComponentHit`
  (params (HitComponent :type "PrimitiveComponent Object Reference") (OtherActor :type "Actor Object Reference") (OtherComp :type "PrimitiveComponent Object Reference") (NormalImpulse :type "Vector Structure") (Hit :type "HitResult Structure (by ref)"))
  ;[1 1 1] Launch Player and bounce when hit
  (`|ExecutionSequence`
    (:`then_0`
      (bind _asbp_player_character (cast `/Game/Custom/Blueprints/Characters/BP_PlayerCharacter` OtherActor))
      (`Character.UnCrouch` _asbp_player_character)
      (`Character.LaunchCharacter` _asbp_player_character (0.0 0.0 1500.0) false true) ; JumpPad
    )
    (:`then_1`
      (cast `/Game/Custom/Blueprints/Actors/BP_Projectile` OtherActor)))
  (`MaterialInstanceDynamic.SetVectorParameterValue` (`self.Material`) "Position" (`KismetMathLibrary.Conv_VectorToLinearColor` Hit_ImpactPoint))
  (bind (_direction _bounce_curve) (`Timeline|Bounce` :!via `PlayFromStart`)
    (:`Update`
      (`MaterialInstanceDynamic.SetVectorParameterValue` (`self.Material`) "Impact" (`KismetMathLibrary.Conv_VectorToLinearColor` (* Hit_Normal (* _bounce_curve (`self.Bounciness`))))))))

(fn `UserConstructionScript`)