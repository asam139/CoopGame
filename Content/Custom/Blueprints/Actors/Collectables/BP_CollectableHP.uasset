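; BP_CollectableHP is a health pickup that heals the player by HealAmount.
; Every Tick it spins the actor and plays a Sway timeline whose curve drives a local offset.
; Tick also polls for overlap with the player pawn, raising the stat through BPCPlayerStats and destroying itself only if that stat is below max.
; An older, disconnected version using PlayerHP variables on ThirdPersonCharacter remains in the graph.
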(event `self.ReceiveTick`
  (params (DeltaSeconds :type "Float (single-precision)"))
  (bind _returnvalue (`GameplayStatics.GetPlayerPawn` 0))
  ;[1 1 1] Animation
  (`|ExecutionSequence`
    (:`then_0`
      (`self.K2_AddActorLocalRotation` (struct :`Yaw` 0.2))
      (bind (_direction _sway_curve) (`Timeline|Sway`)
        (:`Update`
          (`self.K2_AddActorLocalOffset` _sway_curve))))
    (:`then_1`
      ;[1 1 1] Heal Player for 'HealAmount' if 'CurrentValue' != 'MaxValue'
      (if (`self.IsOverlappingActor` _returnvalue)
        (bind _asthird_person_character (cast `/Game/ThirdPersonBP/Blueprints/ThirdPersonCharacter` _returnvalue))
        (bind _bpc_playerstats (`/Game/ThirdPersonBP/Blueprints/ThirdPersonCharacter.BPC_PlayerStats` _asthird_person_character))
        (bind (_statvalue _currentvalue) (`/Game/Custom/Blueprints/Classes/BPC_Master_StatManager.GetStat` _bpc_playerstats "NewEnumerator1"))
        (if (< _currentvalue (`.MaxValue_6_78BD2358461F9A5BB51C0C8C9F4AB9B5` (break `/Game/Custom/Blueprints/Structures/S_StatValue` _statvalue)))
          (`/Game/Custom/Blueprints/Classes/BPC_Master_StatManager.ModifyStat` _bpc_playerstats "NewEnumerator1" (`self.HealAmount`))
          (`self.K2_DestroyActor`))))))

(fn `UserConstructionScript`)